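; Enemy spawner that places BP_BlenderCube actors at its own transform on a looping timer while Spawning is on and fewer than 20 exist.
; Each spawn reads the player's maxHp upgrade to scale enemy damage and HP, and restarts the timer so higher maxHp means faster spawns.
; A random tier makes bigger cubes slower, tougher and harder-hitting.
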(event `self.ReceiveBeginPlay`
  (bind _returnvalue (`KismetSystemLibrary.K2_SetTimer` null "spawn" (`self.timer time`) true))
  (set `self.timer` _returnvalue))

(fn `NewFunction`
  (params (k :type Integer))
  (returns (StructOut :type "/Game/Structs/EnemyStruct Structure (by ref)"))
  (bind _output_get (set `self.param` (`KismetMathLibrary.RandomIntegerInRange` 1 6)))
  (bind _structout (setmembers `/Game/Structs/EnemyStruct` :`StructRef` (`self.stats`) :`speed` (/ 5 (/ (`KismetMathLibrary.Conv_IntToDouble` _output_get) 1.0)) :`size` (* _output_get 0.4) :`damage` (* _output_get k) :`hp` (* _output_get 3 k)))
  (return _structout))

(fn `set spawn`
  (params (spawning :type Boolean))
  (set `self.spawning` spawning))

(fn `set timer`
  (params (Time :type "Float (single-precision)"))
  (`KismetSystemLibrary.K2_ClearAndInvalidateTimerHandle` (`self.timer`))
  (bind _returnvalue (`KismetSystemLibrary.K2_SetTimer` null "spawn" Time true))
  (set `self.timer` _returnvalue))

(fn `spawn`
  (if (`self.spawning`)
    (bind _outactors (`GameplayStatics.GetAllActorsOfClass` "/Game/Blueprints/BP_BlenderCube.BP_BlenderCube_C"))
    (bind _returnvalue (`GameplayStatics.GetActorOfClass` "/Game/FirstPerson/Blueprints/BP_FirstPersonCharacter.BP_FirstPersonCharacter_C"))
    (if (not (>= (`KismetArrayLibrary.Array_Length` _outactors) 20))
      (bind (_upgrades_maxamm _upgrades_multishoot _upgrades_maxhp) (break `/Game/Structs/UpgradesStruct` (`/Game/FirstPerson/Blueprints/BP_FirstPersonCharacter.Upgrades` _returnvalue)))
      (bind _returnvalue_2 (/ _upgrades_maxhp 10))
      (bind _structout (`self.NewFunction` _returnvalue_2))
      (`self.set timer` (/ (`KismetMathLibrary.Conv_IntToDouble` 100) (* _returnvalue_2 10)))
      (`|SpawnActorFromClass` "/Game/Blueprints/BP_BlenderCube.BP_BlenderCube_C" (`SceneComponent.K2_GetComponentToWorld` (`self.DefaultSceneRoot`)) "Undefined" "MultiplyWithRoot" null _structout null))))

(fn `UserConstructionScript`)