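; BP_BlenderCube is an enemy character that chases the player, hops on a timer and splits when killed.
; Its Stats struct sets scale and walk speed, and projectile overlaps subtract HP with a brief hit-material flash.
; On death it rolls a randomized money, ammo and health drop, omitting health when the player is at max.
; Large enough cubes also spawn two smaller, faster copies with reduced stats.
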(event `self.ReceiveTick`
  (params (DeltaSeconds :type "Float (single-precision)"))
  ;[1 1 1] movement
  (`|AIMoveTo` self (0.0 0.0 0.0) (`GameplayStatics.GetPlayerCharacter` 0)))

(event `self.Box.OnComponentBeginOverlap`
  (params (OverlappedComponent :type "PrimitiveComponent Object Reference") (OtherActor :type "Actor Object Reference") (OtherComp :type "PrimitiveComponent Object Reference") (OtherBodyIndex :type Integer) (bFromSweep :type Boolean) (SweepResult :type "HitResult Structure (by ref)"))
  (bind (_speed _size _damage _hp) (break `/Game/Structs/EnemyStruct` (`self.Stats`)))
  (bind _returnvalue (`KismetMathLibrary.Conv_VectorToTransform` (`self.K2_GetActorLocation` self)))
  (bind _returnvalue_2 (* _size 0.5))
  (bind _returnvalue_3 (* _speed 2.0))
  (bind _returnvalue_4 (+ (/ _damage 2) 1))
  (bind _returnvalue_5 (+ (/ _hp 2) 1))
  ;[1 1 1] Killing/multiplying
  (bind _asbp_first_person_projectile (cast `/Game/FirstPerson/Blueprints/BP_FirstPersonProjectile` OtherActor))
  (`PrimitiveComponent.SetMaterial` (`self.121212`) 1 "/Game/Materials/hitCube.hitCube")
  (bind _returnvalue_6 (- _hp (`/Game/FirstPerson/Blueprints/BP_FirstPersonProjectile.Damage` _asbp_first_person_projectile)))
  (setmembers `/Game/Structs/EnemyStruct` :`StructRef` (`self.Stats`) :`hp` _returnvalue_6)
  (if (<= _returnvalue_6 -1)
    (`self.K2_DestroyActor` _asbp_first_person_projectile)
    (bind (_inventory_money _inventory_amm _inventory_hp) (break `/Game/Structs/LootStruct` (`/Game/FirstPerson/Blueprints/BP_FirstPersonCharacter.Inventory` (stale `self.ReceiveBeginPlay` _returnvalue))))
    (bind (_upgrades_maxamm _upgrades_multishoot _upgrades_maxhp) (break `/Game/Structs/UpgradesStruct` (`/Game/FirstPerson/Blueprints/BP_FirstPersonCharacter.Upgrades` (stale `self.ReceiveBeginPlay` _returnvalue))))
    (`self.spawn loot` _returnvalue (== _inventory_hp _upgrades_maxhp))
    (if (>= _size 1)
      (`|SpawnActorFromClass` "BP_BlenderCube_C" _returnvalue "Undefined" "MultiplyWithRoot" null (make `/Game/Structs/EnemyStruct` _returnvalue_3 _returnvalue_2 _returnvalue_4 _returnvalue_5) null)
      (`|SpawnActorFromClass` "BP_BlenderCube_C" _returnvalue "Undefined" "MultiplyWithRoot" null (make `/Game/Structs/EnemyStruct` _returnvalue_3 _returnvalue_2 _returnvalue_4 _returnvalue_5) null)
      (`self.K2_DestroyActor`)
      (else
        (`self.K2_DestroyActor`)))
    (else
      (`KismetSystemLibrary.K2_SetTimerDelegate` (delegate `chng mtrl`) 0.2))))

(event `self.ReceiveBeginPlay`
  (bind _charactermovement (`self.CharacterMovement`))
  (bind (_speed _size _damage _hp) (break `/Game/Structs/EnemyStruct` (`self.Stats`)))
  ;[1 1 1] Constructor
  (bind _returnvalue (`GameplayStatics.GetActorOfClass` "/Game/FirstPerson/Blueprints/BP_FirstPersonCharacter.BP_FirstPersonCharacter_C"))
  (`self.K2_AddActorLocalTransform` (`KismetMathLibrary.MakeTransform` (0.0 0.0 0.0) (struct) (* _size (`self.GetActorScale3D` self))))
  (set `CharacterMovementComponent.MaxWalkSpeed` (* (`CharacterMovementComponent.MaxWalkSpeed` _charactermovement) _speed) _charactermovement)
  (`KismetSystemLibrary.K2_SetTimer` null "jump2" 0.5 true))

(event `chng mtrl`
  ;[1 1 1] Killing/multiplying
  (`PrimitiveComponent.SetMaterial` (`self.121212`) 1 "/Game/FPWeapon/Materials/BaseMaterial.BaseMaterial"))

(fn `jump2`
  (`self.Jump`))

(fn `spawn loot`
  (params (SpawnTransform :type "Transform Structure") (`hp max` :type Boolean))
  (bind _arr (`self.arr`))
  (for _index (range 3)
    (bind _output_get (set `self.randomval` (`KismetMathLibrary.RandomIntegerInRange` -3 6)))
    (if (== _index 2)
      (set `self.randomval` (- _output_get 2)))
    (if (< _output_get 0)
      (`KismetArrayLibrary.Array_Set` _arr _index)
      (else
        (`KismetArrayLibrary.Array_Set` _arr _index (`self.randomval`)))))
  (bind _structout (setmembers `/Game/Structs/LootStruct` :`StructRef` (`self.Drop`) :`money` (* (`|GetArrayItem` _arr) 3) :`amm` (* (`|GetArrayItem` _arr 1) 5) :`hp` (`|GetArrayItem` _arr 2)))
  (if `hp max`
    (bind _structout_2 (setmembers `/Game/Structs/LootStruct` :`StructRef` _structout :`hp` 0)))
  (bind (_money _amm _hp) (break `/Game/Structs/LootStruct` _structout_2))
  (if (not (and (== _money 0) (== _amm 0) (== _hp 0)))
    (`|SpawnActorFromClass` "/Game/Blueprints/BP_drop.BP_drop_C" SpawnTransform "Undefined" "MultiplyWithRoot" null _structout_2 null)))

(fn `UserConstructionScript`)